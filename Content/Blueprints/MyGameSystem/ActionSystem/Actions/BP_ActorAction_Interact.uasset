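; Actor action in the game's action system that makes the controlled actor perform an interaction.
; When its event starts, the server gets the actor's interaction component through an interface message and calls Interact on it if valid.
; The server also locks a BP_MyGameSystemCharacter's input when the action starts and unlocks it when the action ends.
; A MulticastFunctionBody macro separates server-only logic from common logic, which runs the parent's end handling afterwards.
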(event `self.OnEventStarted`
  (`parent.OnEventStarted`)
  (`/AdvancedObjectPlugin/BML_AdvancedObject.MulticastFunctionBody`
    (:`Server`
      (bind _returnvalue (message `InteractingActorInterface.GetInteractionComponent` (`self.GetControlledActor`)))
      (`/Engine/EditorBlueprintResources/StandardMacros.IsValid` _returnvalue
        (:`Is Valid`
          (`InteractionComponent.Interact` _returnvalue))))))

(event `self.OnActionStarted`
  (`parent.OnActionStarted`)
  (`/AdvancedObjectPlugin/BML_AdvancedObject.MulticastFunctionBody`
    (:`Server`
      (bind _asbp_my_game_system_character (cast `/Game/Blueprints/MyGameSystem/Character/BP_MyGameSystemCharacter` (`self.GetControlledActor`)))
      (`/Game/Blueprints/MyGameSystem/Character/BP_MyGameSystemCharacter.LockInput` _asbp_my_game_system_character))))

(event `self.OnActionEnded`
  (`/AdvancedObjectPlugin/BML_AdvancedObject.MulticastFunctionBody`
    (:`Server`
      (bind _asbp_my_game_system_character (cast `/Game/Blueprints/MyGameSystem/Character/BP_MyGameSystemCharacter` (`self.GetControlledActor`)))
      (`/Game/Blueprints/MyGameSystem/Character/BP_MyGameSystemCharacter.UnlockInput` _asbp_my_game_system_character))
    (:`CommonAfter`
      (`parent.OnActionEnded`))))