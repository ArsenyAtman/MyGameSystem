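; BP_TestActor is a test actor that demonstrates changing a UObject's Outer at runtime.
; On BeginPlay it constructs a BP_TestObject and prints the object's Outer and name.
; It then calls the object's ChangeOuter with the level and prints both again, exposing the effect of the re-parenting.
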(event `self.ReceiveBeginPlay`
  (bind _returnvalue (`|GenericCreateObject` "/Game/Blueprints/MyGameSystem/AdvancedObject/BP_TestObject.BP_TestObject_C"))
  (`KismetSystemLibrary.PrintString` (`KismetSystemLibrary.GetDisplayName` (`KismetSystemLibrary.GetOuterObject` _returnvalue)))
  (`KismetSystemLibrary.PrintString` (`KismetSystemLibrary.GetObjectName` _returnvalue))
  (`AdvancedObject.ChangeOuter` _returnvalue (`self.GetLevel`))
  (`KismetSystemLibrary.PrintString` (`KismetSystemLibrary.GetObjectName` _returnvalue))
  (`KismetSystemLibrary.PrintString` (`KismetSystemLibrary.GetDisplayName` (`KismetSystemLibrary.GetOuterObject` _returnvalue))))

(fn `UserConstructionScript`)