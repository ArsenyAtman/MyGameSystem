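; BP_WidgetText is an actor that shows a configurable text string through a W_Text widget component.
; Both the Construction Script and BeginPlay cast the component's widget to W_Text and set its text block to the Text variable.
; This applies the text at construction and again when play begins.
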(event `self.ReceiveBeginPlay`
  (bind _asw_text (cast `/Game/Blueprints/MyGameSystem/Misc/W_Text` (`WidgetComponent.GetWidget` (`self.Widget`))))
  (`TextBlock.SetText` (`/Game/Blueprints/MyGameSystem/Misc/W_Text.TextBlock_30` _asw_text) (`self.Text`)))

(fn `UserConstructionScript`
  (bind _asw_text (cast `/Game/Blueprints/MyGameSystem/Misc/W_Text` (`WidgetComponent.GetWidget` (`self.Widget`))))
  (`TextBlock.SetText` (`/Game/Blueprints/MyGameSystem/Misc/W_Text.TextBlock_30` _asw_text) (`self.Text`)))