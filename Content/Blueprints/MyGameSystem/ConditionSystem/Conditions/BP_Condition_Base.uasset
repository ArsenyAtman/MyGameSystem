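; Base Blueprint condition for the condition system, holding behavior that specific conditions of a controlled actor can share.
; Its Death event constructs a BP_Condition_Dead through the condition component and switches to it.
; A helper returns the controlled actor cast to Character.
; Debug handlers print condition names on start and end, but the nodes binding them are unconnected and BeginPlay is empty.
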(event `Death`
  (bind _returnvalue (`|GenericCreateObject` (`self.GetConditionComponent`) "/Game/Blueprints/MyGameSystem/ConditionSystem/Conditions/BP_Condition_Dead.BP_Condition_Dead_C"))
  (`self.ChangeCondition` _returnvalue))

(event `self.BeginPlay`)

(event `ConditionStart` :!signature `self.OnConditionStarted`
  (params (Condition :type "Condition Object Reference"))
  (`KismetSystemLibrary.PrintString` (`KismetSystemLibrary.GetDisplayName` Condition) true true (struct :`R` 0.165773 :`G` 1.0 :`A` 1.0)))

(event `ConditionEnd` :!signature `self.OnConditionEnded`
  (params (Condition :type "Condition Object Reference"))
  (`KismetSystemLibrary.PrintString` (`KismetSystemLibrary.GetDisplayName` Condition) true true (struct :`R` 1.0 :`A` 1.0)))

(fn `Get Controlled Character`
  (returns (ControlledCharacter :type "Character Object Reference"))
  (return (cast `Character` (`self.GetControlledActor`) :!pure true)))