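; BP_PlayerControllerAdvanced is a player controller that relays player action inputs to the pawn it controls.
; Handler events for jump start and end, crouch, interact, emote and two combos each send a matching message to the controlled pawn.
; The controller holds no action logic itself, leaving each response to the pawn.
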(event `HandleStartJumpingInput`
  (message `/Game/Blueprints/MyGameSystem/Character/BPI_PlayerControllable.InputStartJumping` (`self.K2_GetPawn`)))

(event `HandleEndJumpingInput`
  (message `/Game/Blueprints/MyGameSystem/Character/BPI_PlayerControllable.InputEndJumping` (`self.K2_GetPawn`)))

(event `HandleCrouchInput`
  (message `/Game/Blueprints/MyGameSystem/Character/BPI_PlayerControllable.InputCrouch` (`self.K2_GetPawn`)))

(event `HandleInteractInput`
  (message `/Game/Blueprints/MyGameSystem/Character/BPI_PlayerControllable.InputInteract` (`self.K2_GetPawn`)))

(event `HandleEmoteInput`
  (message `/Game/Blueprints/MyGameSystem/Character/BPI_PlayerControllable.InputEmote` (`self.K2_GetPawn`)))

(event `HandleCombo1Input`
  (message `/Game/Blueprints/MyGameSystem/Character/BPI_PlayerControllable.InputCombo1` (`self.K2_GetPawn`)))

(event `HandleCombo2Input`
  (message `/Game/Blueprints/MyGameSystem/Character/BPI_PlayerControllable.InputCombo2` (`self.K2_GetPawn`)))

(fn `UserConstructionScript`)