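; BP_NPC is a talkable NPC character: it always accepts interaction, labels the action "talk", and starts a dialogue with the interacting actor.
; Dialogue runs through its DialogComponentNPC, with no additional interlocutors passed in.
; Getter functions expose that component, a dialog wave player and a montage player, plus the Mesh and its "head" point as the mouth location and montage target.
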(event `InteractableActorInterface.Interact`
  (params (Actor :type "Actor Object Reference"))
  (`DialogComponent.BeginDialogue` (`self.DialogComponent_NPC`) Actor (`|MakeArray`)))

(fn `CanInteract`
  (params (Actor :type "Actor Object Reference"))
  (returns (ReturnValue :type Boolean))
  (return true))

(fn `GetActionDescription`
  (returns (ReturnValue :type Text))
  (return "talk"))

(fn `GetDialogComponent`
  (returns (ReturnValue :type "DialogComponent Object Reference"))
  (return (`self.DialogComponent_NPC`)))

(fn `GetDialogWavePlayerComponent`
  (returns (ReturnValue :type "DialogWavePlayerComponent Object Reference"))
  (return (`self.DialogWavePlayer`)))

(fn `GetMontagePlayerComponent`
  (returns (ReturnValue :type "MontagePlayerComponent Object Reference"))
  (return (`self.MontagePlayer`)))

(fn `GetMouthComponent`
  (returns (ReturnValue :type "SceneComponent Object Reference"))
  (return (`self.Mesh`)))

(fn `GetMouthPoint`
  (returns (ReturnValue :type Name))
  (return "head"))

(fn `GetMouthRelativeLocation`
  (returns (ReturnValue :type "Vector Structure"))
  (return (0.0 0.0 0.0)))

(fn `GetSkeletalMeshForMontagePlaying`
  (returns (ReturnValue :type "SkeletalMeshComponent Object Reference"))
  (return (`self.Mesh`)))

(fn `UserConstructionScript`)