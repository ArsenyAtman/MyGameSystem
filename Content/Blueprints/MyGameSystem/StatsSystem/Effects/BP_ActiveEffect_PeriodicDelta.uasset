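; Active stat effect that repeatedly applies a Delta to its related stats while it is active.
; On activation it starts a looping timer that calls ApplyDelta every Period, so the first change lands one Period later.
; A positive Duration also schedules deactivation slightly after that time; otherwise the effect runs until deactivated elsewhere.
; Deactivation clears the periodic timer.
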(event `self.OnActivated`
  (bind _duration (`self.Duration`))
  (`parent.OnActivated`)
  (`KismetSystemLibrary.K2_SetTimer` self (`self.ApplyDeltaFunctionName`) (`self.Period`) true)
  (if (> _duration 0.0)
    (`KismetSystemLibrary.K2_SetTimerDelegate` (delegate `DeactivateEffect`) (+ _duration 0.1))))

(event `ApplyDelta`
  (`self.ApplyDeltaToRelatedStats` (make `StatValues` (`self.Delta`))))

(event `DeactivateEffect`
  (`self.Deactivate`))

(event `self.OnDeactivating`
  (`KismetSystemLibrary.K2_ClearTimer` self (`self.ApplyDeltaFunctionName`))
  (`parent.OnDeactivating`))