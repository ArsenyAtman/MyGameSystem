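; Stats-system active effect for stamina usage that swaps out stamina regeneration while it is active.
; On activation, the server aborts the first active StaminaRegen effect on the related stats component.
; On deactivation, the server constructs and applies a fresh StaminaRegen effect for the Stamina stat, then the parent deactivation runs on the common path.
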(event `self.OnActivated`
  (bind _returnvalue (`self.GetRelatedStatsComponent`))
  (`parent.OnActivated`)
  (`/AdvancedObjectPlugin/BML_AdvancedObject.MulticastFunctionBody`
    (:`Server`
      (`StatsComponent.AbortEffect` _returnvalue (`|GetArrayItem` (`StatsComponent.GetEffectsOfClass` _returnvalue "/Game/Blueprints/MyGameSystem/StatsSystem/Effects/BP_ActiveEffect_StaminaRegen.BP_ActiveEffect_StaminaRegen_C"))))))

(event `self.OnDeactivating`
  (bind _returnvalue (`self.GetRelatedStatsComponent`))
  (`/AdvancedObjectPlugin/BML_AdvancedObject.MulticastFunctionBody`
    (:`Server`
      (bind _returnvalue_2 (`|GenericCreateObject` _returnvalue "/Game/Blueprints/MyGameSystem/StatsSystem/Effects/BP_ActiveEffect_StaminaRegen.BP_ActiveEffect_StaminaRegen_C" 5.0 -1.0 1.0 "SearchByNameAndByClass" "/Game/Blueprints/MyGameSystem/StatsSystem/Stats/BP_Stat_Stamina.BP_Stat_Stamina_C" "None"))
      (`StatsComponent.ApplyEffect` _returnvalue _returnvalue_2))
    (:`CommonAfter`
      (`parent.OnDeactivating`))))