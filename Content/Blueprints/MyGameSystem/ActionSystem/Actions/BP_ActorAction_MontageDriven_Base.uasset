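; Base montage-driven actor action that supplies its animation montage and decides how newly attempted actions chain from or interrupt it.
; During an open combo window, ComboMap swaps the attempted action's class for a follow-up, constructed on the action driver component.
; Any other attempt disables further combo input and is filtered by InterruptionType against ListOfActions.
; An accepted action ends this one and starts through the driver component.
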(event `self.NewActionTriedToStart`
  (params (NewAction :type "ActorAction Object Reference"))
  (bind (_value _returnvalue) (`BlueprintMapLibrary.Map_Find` (`self.ComboMap`) (`GameplayStatics.GetObjectClass` NewAction)))
  (bind _returnvalue_2 (!= (`KismetArrayLibrary.Array_Find` (`self.ListOfActions`) (`GameplayStatics.GetObjectClass` NewAction)) -1))
  (if (and (`self.bComboWindowStarted`) (not (`self.IgnoreComboInput`)))
    ;[1 1 1] Combinations
    (if _returnvalue
      (bind _returnvalue_3 (`|GenericCreateObject` _value (`self.GetActionDriverComponent`)))
      (`self.StartNewAction` _returnvalue_3)
      (else
        (set `self.IgnoreComboInput` true :!label _label)
        ;[1 1 1] Interruption
        (switch `/Game/Blueprints/MyGameSystem/ActionSystem/Actions/ActionInterruptionType` (`self.InterruptionType`)
          (:`NewEnumerator0`
            (if _returnvalue_2
              (`self.StartNewAction` NewAction)))
          (:`NewEnumerator1`
            (if (not _returnvalue_2)
              (`self.StartNewAction` NewAction))))))
    (else
      (goto _label))))

(fn `GetAnimationMontageToPlay`
  (returns (ReturnValue :type "AnimMontage Object Reference"))
  (return (`self.MontageToPlay`)))

(fn `StartNewAction`
  (params (NewAction :type "ActorAction Object Reference"))
  (`self.EndAction`)
  (`ActionDriverComponent.StartAction` (`self.GetActionDriverComponent`) NewAction))