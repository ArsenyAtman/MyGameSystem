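; BP_Objective_Base is a quest objective base Blueprint that manages the pickup interactables tied to an objective.
; On activation it casts the quest's related actors to BP_Interactable_Pickup, then shows each one and binds its OnPickedUp event.
; Completion and failure share one cleanup path that unbinds the event and hides those pickups.
; The OnPickedUp handler is empty here, so this asset defines no progress logic.
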(event `self.OnObjectiveActivated`
  (for _array_element (`.RelatedActors` (break `ReferencesForQuest` (`self.ReferencesForQuest`)))
    (bind _asbp_interactable_pickup (cast `/Game/Blueprints/MyGameSystem/InteractionSystem/Interactables/BP_Interactable_Pickup` _array_element))
    (`/Game/Blueprints/MyGameSystem/InteractionSystem/Interactables/BP_Interactable_Pickup.Show` _asbp_interactable_pickup)
    (add `/Game/Blueprints/MyGameSystem/InteractionSystem/Interactables/BP_Interactable_Pickup.OnPickedUp` _asbp_interactable_pickup (delegate `OnPickedUp`))))

(event `OnPickedUp`)

(event `self.OnObjectiveCompleted`
  (for _array_element (`.RelatedActors` (break `ReferencesForQuest` (`self.ReferencesForQuest`))) :!label _label
    (bind _asbp_interactable_pickup (cast `/Game/Blueprints/MyGameSystem/InteractionSystem/Interactables/BP_Interactable_Pickup` _array_element))
    (remove `/Game/Blueprints/MyGameSystem/InteractionSystem/Interactables/BP_Interactable_Pickup.OnPickedUp` _asbp_interactable_pickup (delegate `OnPickedUp`))
    (`/Game/Blueprints/MyGameSystem/InteractionSystem/Interactables/BP_Interactable_Pickup.Hide` _asbp_interactable_pickup)))

(event `self.OnObjectiveFailed`
  (goto _label))