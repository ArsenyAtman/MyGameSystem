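; BP_Interactable_QuestGiver is an interactable actor that hands a quest to whoever interacts with it.
; On Interact it calls the parent, gets the interacting actor's quest component through an interface message and adds the hardcoded BP_Quest_Test1 quest.
; It overrides the action description as "get a quest" and always allows interaction.
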(event `InteractableActorInterface.Interact`
  (params (Actor :type "Actor Object Reference"))
  (`parent.Interact` Actor)
  (bind _returnvalue (message `ActorWithQuestsInterface.GetActorQuestComponent` Actor))
  (`QuestComponent.AddQuest` _returnvalue "/Game/Blueprints/MyGameSystem/QuestSystem/Quests/BP_Quest_Test1.BP_Quest_Test1_C"))

(fn `CanInteract`
  (params (Actor :type "Actor Object Reference"))
  (returns (ReturnValue :type Boolean))
  (return true))

(fn `GetActionDescription`
  (returns (ReturnValue :type Text))
  (return "get a quest"))

(fn `UserConstructionScript`
  (`parent.UserConstructionScript`))