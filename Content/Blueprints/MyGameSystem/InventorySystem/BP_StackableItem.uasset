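; BP_StackableItem is an inventory item actor that can be picked up from the world.
; Interacting gets the actor's inventory manager through an interface message and passes the item to PickupItem.
; The "Pickup" action is allowed only while the item has no valid possessing place.
; When its instanced state changes, it shows or hides its component hierarchy and toggles the Cube's collision to match.
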(event `InteractableActorInterface.Interact`
  (params (Actor :type "Actor Object Reference"))
  (bind _returnvalue (message `ActorWithInventoryInterface.GetInventoryManagerComponent` Actor))
  (`InventoryManagerComponent.PickupItem` _returnvalue self))

(event `self.IsInstancedChanged`
  (`SceneComponent.SetVisibility` (`self.DefaultSceneRoot`) (`self.bIsInstanced`) true)
  (`PrimitiveComponent.SetCollisionEnabled` (`self.Cube`) (select `bool` (`self.bIsInstanced`) :`false` "NoCollision" :`true` "QueryAndPhysics" :!type "ECollisionEnabled Enum")))

(fn `CanInteract`
  (params (Actor :type "Actor Object Reference"))
  (returns (ReturnValue :type Boolean))
  (return (not (`KismetSystemLibrary.IsValid` (`self.GetPossessingPlace`)))))

(fn `GetActionDescription`
  (returns (ReturnValue :type Text))
  (return "Pickup"))

(fn `UserConstructionScript`)