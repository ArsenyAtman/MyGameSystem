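; Crouching condition in the MyGameSystem condition system, representing the controlled character's crouched state.
; On start it sets the character's movement mode to Walking and calls ClientCrouch on BP_MyGameSystemCharacter, then calls ClientUnCrouch when it ends.
; Crouch input constructs a new Standing condition owned by the condition component and switches to it, so crouch acts as a toggle out of this state.
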(event `self.OnConditionStarted`
  (`CharacterMovementComponent.SetMovementMode` (`Character.CharacterMovement` (`self.Get Controlled Character`)) "MOVE_Walking" 0)
  (bind _asbp_my_game_system_character (cast `/Game/Blueprints/MyGameSystem/Character/BP_MyGameSystemCharacter` (`self.Get Controlled Character`)))
  (`/Game/Blueprints/MyGameSystem/Character/BP_MyGameSystemCharacter.ClientCrouch` _asbp_my_game_system_character))

(event `self.OnConditionEnded`
  (bind _asbp_my_game_system_character (cast `/Game/Blueprints/MyGameSystem/Character/BP_MyGameSystemCharacter` (`self.Get Controlled Character`)))
  (`/Game/Blueprints/MyGameSystem/Character/BP_MyGameSystemCharacter.ClientUnCrouch` _asbp_my_game_system_character))

(event `/Game/Blueprints/MyGameSystem/Character/BPI_PlayerControllable.InputCrouch`
  (bind _returnvalue (`|GenericCreateObject` "/Game/Blueprints/MyGameSystem/ConditionSystem/Conditions/BP_Condition_Standing.BP_Condition_Standing_C" (`self.GetConditionComponent`)))
  (`self.ChangeCondition` _returnvalue))