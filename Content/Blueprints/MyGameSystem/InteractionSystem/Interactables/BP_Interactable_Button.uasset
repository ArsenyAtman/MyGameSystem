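; BP_Interactable_Button is a pressable button for the interaction system, always interactable and described as "press the button".
; Interact fires ButtonPress, which plays a chime at the ring mesh and runs a timeline that moves the push mesh along its relative Z.
; It then passes the interacting actor to ButtonLogic, an empty function here that separates the button's effect from its press feedback.
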(event `InteractableActorInterface.Interact`
  (params (Actor :type "Actor Object Reference"))
  (`self.ButtonPress`)
  (`self.ButtonLogic` Actor))

(event `ButtonPress`
  (`GameplayStatics.PlaySoundAtLocation` "/Game/Assets/SFX/SFX_Chime_04A.SFX_Chime_04A" (`SceneComponent.K2_GetComponentLocation` (`self.SM_Button_Ring`)) (struct) 1.0 1.0 0.0 "/Game/Assets/SFX/DefaultSoundAttenuation.DefaultSoundAttenuation" null null)
  (bind (_direction _leverposition) (`Timeline|Timeline_0` :!via `PlayFromStart`)
    (:`Update`
      (`SceneComponent.K2_SetRelativeLocation` (`self.SM_Button_Push`) (`KismetMathLibrary.MakeVector` 0.0 0.0 _leverposition) false false))))

(fn `ButtonLogic`
  (params (Actor :type "Actor Object Reference")))

(fn `CanInteract`
  (params (Actor :type "Actor Object Reference"))
  (returns (ReturnValue :type Boolean))
  (return true))

(fn `GetActionDescription`
  (returns (ReturnValue :type Text))
  (return "press the button"))

(fn `UserConstructionScript`)