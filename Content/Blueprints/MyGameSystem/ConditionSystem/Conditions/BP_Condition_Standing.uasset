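; Standing condition in the character condition system, the state for normal on-foot movement that sets the server's movement mode to Walking when it starts.
; Crouch input switches to the Crouching condition, and jump input either jumps or, while falling, switches to the Flying condition.
; Interact, emote and combo inputs construct action objects and start them on the character's action driver component, with interact first checking the interaction component.
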(event `self.ConditionStarted`
  (`parent.ConditionStarted`)
  (`/AdvancedObjectPlugin/BML_AdvancedObject.MulticastFunctionBody`
    (:`Server`
      (`CharacterMovementComponent.SetMovementMode` (`Character.CharacterMovement` (`self.Get Controlled Character`)) "MOVE_Walking" 0))))

(event `/Game/Blueprints/MyGameSystem/Character/BPI_PlayerControllable.InputCrouch`
  (bind _returnvalue (`|GenericCreateObject` "/Game/Blueprints/MyGameSystem/ConditionSystem/Conditions/BP_Condition_Crouching.BP_Condition_Crouching_C"))
  (`self.ChangeCondition` _returnvalue))

(event `/Game/Blueprints/MyGameSystem/Character/BPI_PlayerControllable.InputStartJumping`
  (bind _asbp_my_game_system_character (cast `/Game/Blueprints/MyGameSystem/Character/BP_MyGameSystemCharacter` (`self.Get Controlled Character`)))
  (if (`NavMovementComponent.IsFalling` (`Character.CharacterMovement` _asbp_my_game_system_character))
    (bind _returnvalue (`|GenericCreateObject` "/Game/Blueprints/MyGameSystem/ConditionSystem/Conditions/BP_Condition_Flying.BP_Condition_Flying_C"))
    (`self.ChangeCondition` _returnvalue)
    (else
      (`/Game/Blueprints/MyGameSystem/Character/BP_MyGameSystemCharacter.ClientJump` _asbp_my_game_system_character))))

(event `/Game/Blueprints/MyGameSystem/Character/BPI_PlayerControllable.InputEndJumping`
  (bind _asbp_my_game_system_character (cast `/Game/Blueprints/MyGameSystem/Character/BP_MyGameSystemCharacter` (`self.Get Controlled Character`)))
  (`/Game/Blueprints/MyGameSystem/Character/BP_MyGameSystemCharacter.ClientStopJumping` _asbp_my_game_system_character))

(event `/Game/Blueprints/MyGameSystem/Character/BPI_PlayerControllable.InputInteract`
  (bind _returnvalue (message `InteractingActorInterface.GetInteractionComponent` (`self.Get Controlled Character`)))
  (`/Engine/EditorBlueprintResources/StandardMacros.IsValid` _returnvalue
    (:`Is Valid`
      (if (`InteractionComponent.CanInteract` _returnvalue)
        (bind _returnvalue_2 (message `ActionDrivenActorInterface.GetActionDriverComponent` (`self.Get Controlled Character`)))
        (`/Engine/EditorBlueprintResources/StandardMacros.IsValid` _returnvalue_2
          (:`Is Valid`
            (bind _returnvalue_3 (`|GenericCreateObject` "/Game/Blueprints/MyGameSystem/ActionSystem/Actions/BP_ActorAction_Interact.BP_ActorAction_Interact_C"))
            (`ActionDriverComponent.StartAction` _returnvalue_2 _returnvalue_3)))))))

(event `/Game/Blueprints/MyGameSystem/Character/BPI_PlayerControllable.InputEmote`
  (bind _returnvalue (message `ActionDrivenActorInterface.GetActionDriverComponent` (`self.Get Controlled Character`)))
  (`/Engine/EditorBlueprintResources/StandardMacros.IsValid` _returnvalue
    (:`Is Valid`
      (bind _returnvalue_2 (`|GenericCreateObject` "/Game/Blueprints/MyGameSystem/ActionSystem/Actions/BP_ActorAction_Celebrate.BP_ActorAction_Celebrate_C"))
      (`ActionDriverComponent.StartAction` _returnvalue _returnvalue_2))))

(event `/Game/Blueprints/MyGameSystem/Character/BPI_PlayerControllable.InputCombo1`
  (bind _returnvalue (message `ActionDrivenActorInterface.GetActionDriverComponent` (`self.Get Controlled Character`)))
  (`/Engine/EditorBlueprintResources/StandardMacros.IsValid` _returnvalue
    (:`Is Valid`
      (bind _returnvalue_2 (`|GenericCreateObject` "/Game/Blueprints/MyGameSystem/ActionSystem/Actions/BP_ActorAction_Combo1.BP_ActorAction_Combo1_C"))
      (`ActionDriverComponent.StartAction` _returnvalue _returnvalue_2))))

(event `/Game/Blueprints/MyGameSystem/Character/BPI_PlayerControllable.InputCombo2`
  (bind _returnvalue (message `ActionDrivenActorInterface.GetActionDriverComponent` (`self.Get Controlled Character`)))
  (`/Engine/EditorBlueprintResources/StandardMacros.IsValid` _returnvalue
    (:`Is Valid`
      (bind _returnvalue_2 (`|GenericCreateObject` "/Game/Blueprints/MyGameSystem/ActionSystem/Actions/BP_ActorAction_Combo2.BP_ActorAction_Combo2_C"))
      (`ActionDriverComponent.StartAction` _returnvalue _returnvalue_2))))