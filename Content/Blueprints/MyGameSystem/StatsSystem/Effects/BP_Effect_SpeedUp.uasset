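; Timed stats-system effect that temporarily speeds up a BP_MyGameSystemCharacter.
; On activation it adds SpeedDelta to the related character's max walk speed and starts a timer for EffectDuration.
; When the timer fires the effect deactivates itself, and on deactivating it subtracts the same delta from the current speed rather than restoring a saved value.
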(event `self.OnActivated`
  (`parent.OnActivated`)
  (bind _asbp_my_game_system_character (cast `/Game/Blueprints/MyGameSystem/Character/BP_MyGameSystemCharacter` (`self.GetRelatedActor`)))
  (`/Game/Blueprints/MyGameSystem/Character/BP_MyGameSystemCharacter.SetMaxWalkSpeed` _asbp_my_game_system_character (+ (`CharacterMovementComponent.MaxWalkSpeed` (`Character.CharacterMovement` _asbp_my_game_system_character)) (`self.SpeedDelta`)))
  (`KismetSystemLibrary.K2_SetTimerDelegate` (delegate `DeactivateEffect`) (`self.EffectDuration`)))

(event `self.OnDeactivating`
  (bind _asbp_my_game_system_character (cast `/Game/Blueprints/MyGameSystem/Character/BP_MyGameSystemCharacter` (`self.GetRelatedActor`)))
  (`/Game/Blueprints/MyGameSystem/Character/BP_MyGameSystemCharacter.SetMaxWalkSpeed` _asbp_my_game_system_character (- (`CharacterMovementComponent.MaxWalkSpeed` (`Character.CharacterMovement` _asbp_my_game_system_character)) (`self.SpeedDelta`)))
  (`parent.OnDeactivating`))

(event `DeactivateEffect`
  (`self.Deactivate`))