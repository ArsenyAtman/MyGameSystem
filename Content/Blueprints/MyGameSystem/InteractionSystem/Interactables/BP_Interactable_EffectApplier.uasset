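; BP_Interactable_EffectApplier is an interactable that applies an effect to the actor passed into its button logic.
; ButtonLogic gets that actor's stats component through an interface message, constructs an object from EffectClass and passes it to ApplyEffect if the component is valid.
; GetActionDescription supplies the "apply the effect" action text, and the event graph holds only disabled default events.
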(fn `ButtonLogic`
  (params (Actor :type "Actor Object Reference"))
  (bind _returnvalue (message `ActorWithStatsInterface.GetStatsComponent` Actor))
  (`/Engine/EditorBlueprintResources/StandardMacros.IsValid` _returnvalue
    (:`Is Valid`
      (bind _returnvalue_2 (`|GenericCreateObject` (`self.EffectClass`)))
      (`StatsComponent.ApplyEffect` _returnvalue _returnvalue_2))))

(fn `GetActionDescription`
  (returns (ReturnValue :type Text))
  (return "apply the effect"))

(fn `UserConstructionScript`
  (`parent.UserConstructionScript`))