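; Player controller Blueprint that routes Enhanced Input actions to the controlled pawn.
; On BeginPlay it adds the IMC_InputMappingContext mapping context to the local player's input subsystem.
; Jump, crouch, interact, emote and two combo actions each call a handler event that sends a matching message to the pawn, keeping input decoupled from pawn logic.
; Jump splits its action value into separate start and end messages.
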(event `self.ReceiveBeginPlay`
  (bind _returnvalue (subsystem `EnhancedInputLocalPlayerSubsystem`))
  (`/Engine/EditorBlueprintResources/StandardMacros.IsValid` _returnvalue
    (:`Is Valid`
      (`EnhancedInputSubsystemInterface.AddMappingContext` _returnvalue "/Game/Blueprints/MyGameSystem/Input/IMC_InputMappingContext.IMC_InputMappingContext" 0 (struct)))))

(event `HandleStartJumpingInput`
  (message `/Game/Blueprints/MyGameSystem/Character/BPI_PlayerControllable.InputStartJumping` (`self.K2_GetPawn`)))

(event `EnhancedInput|/Game/Blueprints/MyGameSystem/Input/IA_Jump`
  (params (ActionValue :type Boolean) (ElapsedSeconds :type "Float (double-precision)") (TriggeredSeconds :type "Float (double-precision)") (InputAction :type "InputAction Object Reference" :default "/Game/Blueprints/MyGameSystem/Input/IA_Jump.IA_Jump"))
  (:`Triggered`
    (if ActionValue
      (`self.HandleStartJumpingInput`)
      (else
        (`self.HandleEndJumpingInput`)))))

(event `HandleEndJumpingInput`
  (message `/Game/Blueprints/MyGameSystem/Character/BPI_PlayerControllable.InputEndJumping` (`self.K2_GetPawn`)))

(event `HandleCrouchInput`
  (message `/Game/Blueprints/MyGameSystem/Character/BPI_PlayerControllable.InputCrouch` (`self.K2_GetPawn`)))

(event `EnhancedInput|/Game/Blueprints/MyGameSystem/Input/IA_Crouch`
  (params (ActionValue :type Boolean) (ElapsedSeconds :type "Float (double-precision)") (TriggeredSeconds :type "Float (double-precision)") (InputAction :type "InputAction Object Reference" :default "/Game/Blueprints/MyGameSystem/Input/IA_Crouch.IA_Crouch"))
  (:`Triggered`
    (`self.HandleCrouchInput`)))

(event `HandleInteractInput`
  (message `/Game/Blueprints/MyGameSystem/Character/BPI_PlayerControllable.InputInteract` (`self.K2_GetPawn`)))

(event `EnhancedInput|/Game/Blueprints/MyGameSystem/Input/IA_Interact`
  (params (ActionValue :type Boolean) (ElapsedSeconds :type "Float (double-precision)") (TriggeredSeconds :type "Float (double-precision)") (InputAction :type "InputAction Object Reference" :default "/Game/Blueprints/MyGameSystem/Input/IA_Interact.IA_Interact"))
  (:`Triggered`
    (`self.HandleInteractInput`)))

(event `EnhancedInput|/Game/Blueprints/MyGameSystem/Input/IA_Emote`
  (params (ActionValue :type Boolean) (ElapsedSeconds :type "Float (double-precision)") (TriggeredSeconds :type "Float (double-precision)") (InputAction :type "InputAction Object Reference" :default "/Game/Blueprints/MyGameSystem/Input/IA_Emote.IA_Emote"))
  (:`Triggered`
    (`self.HandleEmoteInput`)))

(event `HandleEmoteInput`
  (message `/Game/Blueprints/MyGameSystem/Character/BPI_PlayerControllable.InputEmote` (`self.K2_GetPawn`)))

(event `EnhancedInput|/Game/Blueprints/MyGameSystem/Input/IA_Combo1`
  (params (ActionValue :type Boolean) (ElapsedSeconds :type "Float (double-precision)") (TriggeredSeconds :type "Float (double-precision)") (InputAction :type "InputAction Object Reference" :default "/Game/Blueprints/MyGameSystem/Input/IA_Combo1.IA_Combo1"))
  (:`Triggered`
    (`self.HandleCombo1Input`)))

(event `HandleCombo1Input`
  (message `/Game/Blueprints/MyGameSystem/Character/BPI_PlayerControllable.InputCombo1` (`self.K2_GetPawn`)))

(event `HandleCombo2Input`
  (message `/Game/Blueprints/MyGameSystem/Character/BPI_PlayerControllable.InputCombo2` (`self.K2_GetPawn`)))

(event `EnhancedInput|/Game/Blueprints/MyGameSystem/Input/IA_Combo2`
  (params (ActionValue :type Boolean) (ElapsedSeconds :type "Float (double-precision)") (TriggeredSeconds :type "Float (double-precision)") (InputAction :type "InputAction Object Reference" :default "/Game/Blueprints/MyGameSystem/Input/IA_Combo2.IA_Combo2"))
  (:`Triggered`
    (`self.HandleCombo2Input`)))

(fn `UserConstructionScript`)