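; Player character for MyGameSystem that hosts stats, condition, inventory, quest, dialog, interaction and montage components, exposed through getter functions.
; Jump, crouch, interact, emote and combo inputs forward to the ConditionComponent's current condition, while move and look apply directly.
; On the server it adds stamina with regen and routes the first stat's minimum to the condition's Death, with a separate Death event that ragdolls the mesh.
; Dialog pauses interaction tracing, and inventory connections toggle the HUD on clients.
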(event `EnhancedInput|/Game/Blueprints/MyGameSystem/Input/IA_Move`
  (params (ActionValue :type "Vector2D Structure") (ElapsedSeconds :type "Float (double-precision)") (TriggeredSeconds :type "Float (double-precision)") (InputAction :type "InputAction Object Reference" :default "/Game/Blueprints/MyGameSystem/Input/IA_Move.IA_Move"))
  (bind (_x _y) (`KismetMathLibrary.BreakVector2D` ActionValue))
  (bind _returnvalue (`KismetMathLibrary.MakeRotator` 0.0 0.0 (.yaw (`self.GetControlRotation`))))
  ;[1 1 1] MovementInput
  (:`Triggered`
    (`|ExecutionSequence`
      (:`then_0`
        (`self.AddMovementInput` (`KismetMathLibrary.GetForwardVector` _returnvalue) _y))
      (:`then_1`
        (`self.AddMovementInput` (`KismetMathLibrary.GetRightVector` _returnvalue) _x)))))

(event `EnhancedInput|/Game/Blueprints/MyGameSystem/Input/IA_Look`
  (params (ActionValue :type "Vector2D Structure") (ElapsedSeconds :type "Float (double-precision)") (TriggeredSeconds :type "Float (double-precision)") (InputAction :type "InputAction Object Reference" :default "/Game/Blueprints/MyGameSystem/Input/IA_Look.IA_Look"))
  (bind (_x _y) (`KismetMathLibrary.BreakVector2D` ActionValue))
  ;[1 1 1] ViewInput
  (:`Triggered`
    (`|ExecutionSequence`
      (:`then_0`
        (`self.AddControllerYawInput` _x))
      (:`then_1`
        (`self.AddControllerPitchInput` _y)))))

(event `ClientJump`
  ;[1 1 1] JumpLogic
  (`self.Jump`))

(event `ClientCrouch`
  ;[1 1 1] CrouchLogic
  (`self.Crouch`))

(event `ClientStopJumping`
  ;[1 1 1] JumpLogic
  (`self.StopJumping`))

(event `ClientUnCrouch`
  ;[1 1 1] CrouchLogic
  (`self.UnCrouch`))

(event `self.ReceiveBeginPlay`
  ;[1 1 1] BeginPlay
  (`/Engine/EditorBlueprintResources/ActorMacros.Switch Has Authority`
    (:`Authority`
      (add `Stat.OnMinReached` (`|GetArrayItem` (`StatsComponent.Stats` (`self.StatsComponent`))) (delegate `Die`))
      (bind _returnvalue (`|GenericCreateObject` (`self.StatsComponent`) "/Game/Blueprints/MyGameSystem/StatsSystem/Effects/BP_ActiveEffect_StaminaRegen.BP_ActiveEffect_StaminaRegen_C" 5.0 -1.0 1.0 "/Game/Blueprints/MyGameSystem/StatsSystem/Stats/BP_Stat_Stamina.BP_Stat_Stamina_C"))
      (`EffectsComponent.AddEffect` (`self.StatsComponent`) _returnvalue)
      (bind _returnvalue_2 (`|GenericCreateObject` "/Game/Blueprints/MyGameSystem/StatsSystem/Stats/BP_Stat_Stamina.BP_Stat_Stamina_C"))
      (`StatsComponent.AddStat` (`self.StatsComponent`) _returnvalue_2))))

(event `/Game/Blueprints/MyGameSystem/Character/BPI_PlayerControllable.InputStartJumping`
  ;[1 1 1] PlayerControllable
  (message `/Game/Blueprints/MyGameSystem/Character/BPI_PlayerControllable.InputStartJumping` (`ConditionComponent.CurrentCondition` (`self.ConditionComponent`))))

(event `/Game/Blueprints/MyGameSystem/Character/BPI_PlayerControllable.InputEndJumping`
  ;[1 1 1] PlayerControllable
  (message `/Game/Blueprints/MyGameSystem/Character/BPI_PlayerControllable.InputEndJumping` (`ConditionComponent.CurrentCondition` (`self.ConditionComponent`))))

(event `Die`
  (params (Stat :type "Stat Object Reference") (PrevValues :type "StatValues Structure"))
  ;[1 1 1] DeathLogic
  (bind _asbp_condition_base (cast `/Game/Blueprints/MyGameSystem/ConditionSystem/Conditions/BP_Condition_Base` (`ConditionComponent.CurrentCondition` (`self.ConditionComponent`))))
  (`/Game/Blueprints/MyGameSystem/ConditionSystem/Conditions/BP_Condition_Base.Death` _asbp_condition_base))

(event `/Game/Blueprints/MyGameSystem/Character/BPI_PlayerControllable.InputCrouch`
  ;[1 1 1] PlayerControllable
  (message `/Game/Blueprints/MyGameSystem/Character/BPI_PlayerControllable.InputCrouch` (`ConditionComponent.CurrentCondition` (`self.ConditionComponent`))))

(event `Death`
  (bind _mesh (`self.Mesh`))
  ;[1 1 1] DeathLogic
  (`SkeletalMeshComponent.SetAllBodiesBelowSimulatePhysics` _mesh "pelvis" true true)
  (`SkeletalMeshComponent.SetAllBodiesBelowPhysicsBlendWeight` _mesh "pelvis" 1.0 false true)
  (`PrimitiveComponent.SetCollisionProfileName` _mesh "Ragdoll" true)
  (`PrimitiveComponent.SetCollisionProfileName` (`self.CapsuleComponent`) "NoCollision" true))

(event `/Game/Blueprints/MyGameSystem/Character/BPI_PlayerControllable.InputInteract`
  ;[1 1 1] PlayerControllable
  (message `/Game/Blueprints/MyGameSystem/Character/BPI_PlayerControllable.InputInteract` (`ConditionComponent.CurrentCondition` (`self.ConditionComponent`))))

(event `/Game/Blueprints/MyGameSystem/Character/BPI_PlayerControllable.InputEmote`
  ;[1 1 1] PlayerControllable
  (message `/Game/Blueprints/MyGameSystem/Character/BPI_PlayerControllable.InputEmote` (`ConditionComponent.CurrentCondition` (`self.ConditionComponent`))))

(event `/Game/Blueprints/MyGameSystem/Character/BPI_PlayerControllable.InputCombo1`
  ;[1 1 1] PlayerControllable
  (message `/Game/Blueprints/MyGameSystem/Character/BPI_PlayerControllable.InputCombo1` (`ConditionComponent.CurrentCondition` (`self.ConditionComponent`))))

(event `SetMaxWalkSpeed`
  (params (NewMaxWalkSpeed :type "Float (double-precision)"))
  ;[1 1 1] ChangeMaxWalkSpeedReplicated
  (set `CharacterMovementComponent.MaxWalkSpeed` NewMaxWalkSpeed (`self.CharacterMovement`)))

(event `/Game/Blueprints/MyGameSystem/Character/BPI_PlayerControllable.InputCombo2`
  ;[1 1 1] PlayerControllable
  (message `/Game/Blueprints/MyGameSystem/Character/BPI_PlayerControllable.InputCombo2` (`ConditionComponent.CurrentCondition` (`self.ConditionComponent`))))

(event `LockInput`
  (bind _returnvalue (`GameplayStatics.GetPlayerController` 0))
  ;[1 1 1] Lock input while interacting
  (`Controller.SetIgnoreLookInput` _returnvalue true)
  (`Controller.SetIgnoreMoveInput` _returnvalue true))

(event `self.DialogComponent.OnDialogStarted`
  (params (Dialog :type "Dialog Object Reference"))
  ;[1 1 1] Disable tracing in dialog
  (set `InteractionComponent.bIsTracing` false (`self.InteractionComponent`)))

(event `self.DialogComponent.OnDialogEnded`
  (params (Dialog :type "Dialog Object Reference"))
  ;[1 1 1] Disable tracing in dialog
  (set `InteractionComponent.bIsTracing` true (`self.InteractionComponent`)))

(event `UnlockInput`
  (bind _returnvalue (`GameplayStatics.GetPlayerController` 0))
  ;[1 1 1] Lock input while interacting
  (`Controller.SetIgnoreLookInput` _returnvalue false)
  (`Controller.SetIgnoreMoveInput` _returnvalue false))

(event `self.QuestComponent.OnQuestAdded`
  (params (Quest :type "Quest Object Reference"))
  (`/Engine/EditorBlueprintResources/ActorMacros.Switch Has Authority`
    (:`Authority`
      (set `Quest.bIsBeingTracked` true Quest))))

(event `Key|Tab`
  (params (Key :type "Key Structure"))
  (:`Pressed`
    (`/Game/Blueprints/MyGameSystem/UI/BP_MyGameSystemHUD.ShowInventory` (cast `/Game/Blueprints/MyGameSystem/UI/BP_MyGameSystemHUD` (`PlayerController.GetHUD` (`GameplayStatics.GetPlayerController` 0)) :!pure true) true null)))

(event `self.InventoryManager.OnInventoryConnected`
  (params (InventoryManager :type "InventoryManagerComponent Object Reference") (InventoryComponent :type "InventoryComponent Object Reference"))
  (`/Engine/EditorBlueprintResources/ActorMacros.Switch Has Authority`
    (:`Remote`
      (`/Game/Blueprints/MyGameSystem/UI/BP_MyGameSystemHUD.ShowInventory` (cast `/Game/Blueprints/MyGameSystem/UI/BP_MyGameSystemHUD` (`PlayerController.GetHUD` (`GameplayStatics.GetPlayerController` 0)) :!pure true) true InventoryComponent)
      (`KismetSystemLibrary.PrintString` "Hello"))))

(event `self.InventoryManager.OnInventoryDisconnected`
  (params (InventoryManager :type "InventoryManagerComponent Object Reference") (InventoryComponent :type "InventoryComponent Object Reference"))
  (`/Engine/EditorBlueprintResources/ActorMacros.Switch Has Authority`
    (:`Remote`
      (`/Game/Blueprints/MyGameSystem/UI/BP_MyGameSystemHUD.ShowInventory` (cast `/Game/Blueprints/MyGameSystem/UI/BP_MyGameSystemHUD` (`PlayerController.GetHUD` (`GameplayStatics.GetPlayerController` 0)) :!pure true) false null)
      (`KismetSystemLibrary.PrintString` "Bye"))))

(event `Disconnect`
  (bind _inventorymanager (`self.InventoryManager`))
  (`InventoryManagerComponent.Disconnect` _inventorymanager (`|GetArrayItem` (`InventoryManagerComponent.GetConnections` _inventorymanager))))

(fn `GetActionDriverComponent`
  (returns (ReturnValue :type "ActionDriverComponent Object Reference"))
  (return (`self.ActionDriver`)))

(fn `GetActorQuestComponent`
  (returns (ReturnValue :type "QuestComponent Object Reference"))
  (return (`self.QuestComponent`)))

(fn `GetConditionComponent`
  (returns (ReturnValue :type "ConditionComponent Object Reference"))
  (return (`self.ConditionComponent`)))

(fn `GetDialogComponent`
  (returns (ReturnValue :type "DialogComponent Object Reference"))
  (return (`self.DialogComponent`)))

(fn `GetDialogWavePlayerComponent`
  (returns (ReturnValue :type "DialogWavePlayerComponent Object Reference"))
  (return (`self.DialogWavePlayer`)))

(fn `GetDropTransform`
  (returns (ReturnValue :type "Transform Structure"))
  (return (`self.GetTransform`)))

(fn `GetInteractionComponent`
  (returns (ReturnValue :type "InteractionComponent Object Reference"))
  (return (`self.InteractionComponent`)))

(fn `GetInventoryComponent`
  (returns (ReturnValue :type "InventoryComponent Object Reference"))
  (return (`self.Inventory`)))

(fn `GetInventoryManagerComponent`
  (returns (ReturnValue :type "InventoryManagerComponent Object Reference"))
  (return (`self.InventoryManager`)))

(fn `GetMontagePlayerComponent`
  (returns (ReturnValue :type "MontagePlayerComponent Object Reference"))
  (return (`self.MontagePlayer`)))

(fn `GetMouthComponent`
  (returns (ReturnValue :type "SceneComponent Object Reference"))
  (return (`self.CapsuleComponent`)))

(fn `GetMouthPoint`
  (returns (ReturnValue :type Name))
  (return "None"))

(fn `GetMouthRelativeLocation`
  (returns (ReturnValue :type "Vector Structure"))
  (return (0.0 0.0 0.0)))

(fn `GetSkeletalMeshForMontagePlaying`
  (returns (ReturnValue :type "SkeletalMeshComponent Object Reference"))
  (return (`self.Mesh`)))

(fn `GetStatsComponent`
  (returns (ReturnValue :type "StatsComponent Object Reference"))
  (return (`self.StatsComponent`)))

(fn `GetTraceSceneComponent`
  (returns (ReturnValue :type "SceneComponent Object Reference"))
  (return (`self.Camera`)))

(fn `UserConstructionScript`)