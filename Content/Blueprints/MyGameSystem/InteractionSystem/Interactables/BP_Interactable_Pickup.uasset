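; Interactable pickup that spins its static mesh every tick and always allows interaction under a "pick up" prompt.
; It starts hidden without collision on BeginPlay, with a Show event that restores visibility and blocking collision.
; Interacting plays a chime at the mesh, hides it again and fires OnPickedUp.
; It also supplies an interaction marker transform raised above the origin.
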(event `self.ReceiveBeginPlay`
  (`self.Hide`))

(event `Show`
  (bind _staticmesh (`self.StaticMesh`))
  (`SceneComponent.SetHiddenInGame` _staticmesh false true)
  (`PrimitiveComponent.SetCollisionProfileName` _staticmesh "BlockAllDynamic" true)
  (`KismetSystemLibrary.PrintString` "SHOW"))

(event `Hide`
  (bind _staticmesh (`self.StaticMesh`))
  (`SceneComponent.SetHiddenInGame` _staticmesh true true)
  (`PrimitiveComponent.SetCollisionProfileName` _staticmesh "NoCollision" true)
  (`KismetSystemLibrary.PrintString` "HIDE"))

(event `self.ReceiveTick`
  (params (DeltaSeconds :type "Float (single-precision)"))
  (`SceneComponent.K2_SetRelativeRotation` (`self.StaticMesh`) (`KismetMathLibrary.ComposeRotators` (* (`self.RotationSpeed`) DeltaSeconds) (`SceneComponent.RelativeRotation` (`self.StaticMesh`))) false false))

(event `InteractableActorInterface.Interact`
  (params (Actor :type "Actor Object Reference"))
  (`self.Interaction`)
  (`self.OnPickedUp`))

(event `Interaction`
  (`GameplayStatics.PlaySoundAtLocation` "/Game/Assets/SFX/SFX_Chime_03B.SFX_Chime_03B" (`SceneComponent.K2_GetComponentLocation` (`self.StaticMesh`)) (struct) 1.0 1.0 0.0 "/Game/Assets/SFX/DefaultSoundAttenuation.DefaultSoundAttenuation" null null null)
  (`self.Hide`))

(fn `CanInteract`
  (params (Actor :type "Actor Object Reference"))
  (returns (ReturnValue :type Boolean))
  (return true))

(fn `GetActionDescription`
  (returns (ReturnValue :type Text))
  (return "pick up"))

(fn `GetMarkerRelativeTransform`
  (returns (ReturnValue :type "Transform Structure"))
  (return (`KismetMathLibrary.MakeTransform` (0.0 0.0 250.0))))

(fn `UserConstructionScript`)