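; BP_Chest is an interactable chest actor that holds its own Inventory component.
; On BeginPlay it adds two item places, BPItemPlace1 and BPItemPlace2, to that inventory.
; Interacting gets the interacting actor's inventory manager through an interface message and connects it to the chest's Inventory.
; It always allows interaction, supplies the "Open the Chest" prompt, and uses its own transform as the drop transform.
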(event `self.ReceiveBeginPlay`
  (for _array_element (`|MakeArray` (`self.BP_ItemPlace1`) (`self.BP_ItemPlace2`) :!type "ItemPlace Object Reference")
    (`InventoryComponent.AddPlace` (`self.Inventory`) _array_element)))

(event `InteractableActorInterface.Interact`
  (params (Actor :type "Actor Object Reference"))
  (bind _returnvalue (message `ActorWithInventoryInterface.GetInventoryManagerComponent` Actor))
  (`InventoryManagerComponent.Connect` _returnvalue (`self.Inventory`)))

(fn `CanInteract`
  (params (Actor :type "Actor Object Reference"))
  (returns (ReturnValue :type Boolean))
  (return true))

(fn `GetActionDescription`
  (returns (ReturnValue :type Text))
  (return "Open the Chest"))

(fn `GetDropTransform`
  (returns (ReturnValue :type "Transform Structure"))
  (return (`self.GetTransform`)))

(fn `GetInventoryComponent`
  (returns (ReturnValue :type "InventoryComponent Object Reference"))
  (return (`self.Inventory`)))

(fn `GetInventoryManagerComponent`
  (returns (ReturnValue :type "InventoryManagerComponent Object Reference"))
  (return null))

(fn `UserConstructionScript`)