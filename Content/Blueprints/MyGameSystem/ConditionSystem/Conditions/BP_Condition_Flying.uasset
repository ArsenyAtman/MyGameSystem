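; Flying condition for the character condition system that lets the controlled character fly while stamina lasts.
; On start it launches the character forward and up, then after a short timer switches movement to Flying and applies a stamina usage effect.
; Pressing jump or stamina reaching its minimum changes to the Standing condition.
; On end it sets movement to Falling, aborts the stamina effect and unbinds the stamina event.
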(event `self.OnConditionStarted`
  (bind _asbp_my_game_system_character (cast `/Game/Blueprints/MyGameSystem/Character/BP_MyGameSystemCharacter` (`self.Get Controlled Character`)))
  (`Character.LaunchCharacter` _asbp_my_game_system_character (+ (* (`KismetMathLibrary.Normal` (`SceneComponent.GetForwardVector` (`Character.CapsuleComponent` _asbp_my_game_system_character))) 400.0) (0.0 0.0 400.0)) false false)
  (`KismetSystemLibrary.K2_SetTimerDelegate` (delegate `SetModeToFlying`) 0.05))

(event `SetModeToFlying`
  ;[1 1 1] SetModeToFlying
  (`CharacterMovementComponent.SetMovementMode` (`Character.CharacterMovement` (stale `self.OnConditionStarted` _asbp_my_game_system_character)) "MOVE_Flying" 0)
  ;[1 1 1] ApplyStaminaUsageEffect
  (bind _returnvalue (message `ActorWithStatsInterface.GetStatsComponent` (`self.Get Controlled Character`)))
  (`/Engine/EditorBlueprintResources/StandardMacros.IsValid` _returnvalue
    (:`Is Valid`
      (bind _returnvalue_2 (`|GenericCreateObject` "/Game/Blueprints/MyGameSystem/StatsSystem/Effects/BP_ActiveEffect_StaminaUsage.BP_ActiveEffect_StaminaUsage_C" _returnvalue -15.0 -1.0 1.0 "/Game/Blueprints/MyGameSystem/StatsSystem/Stats/BP_Stat_Stamina.BP_Stat_Stamina_C"))
      (bind _output_get (set `self.StaminaUsageEffect` _returnvalue_2))
      (`StatsComponent.ApplyEffect` _returnvalue _output_get)
      (add `Stat.OnMinReached` (`|GetArrayItem` (`StatsComponent.GetStatsOfClass` _returnvalue "/Game/Blueprints/MyGameSystem/StatsSystem/Stats/BP_Stat_Stamina.BP_Stat_Stamina_C")) (delegate `EndCondition`)))))

(event `self.OnConditionEnded`
  (bind _asbp_my_game_system_character (cast `/Game/Blueprints/MyGameSystem/Character/BP_MyGameSystemCharacter` (`self.Get Controlled Character`)))
  (`CharacterMovementComponent.SetMovementMode` (`Character.CharacterMovement` _asbp_my_game_system_character) "MOVE_Falling" 0)
  (bind _returnvalue (message `ActorWithStatsInterface.GetStatsComponent` (`self.Get Controlled Character`)))
  (`/Engine/EditorBlueprintResources/StandardMacros.IsValid` _returnvalue
    (:`Is Valid`
      (`StatsComponent.AbortEffect` _returnvalue (`self.StaminaUsageEffect`))
      (remove `Stat.OnMinReached` (`|GetArrayItem` (`StatsComponent.GetStatsOfClass` _returnvalue "/Game/Blueprints/MyGameSystem/StatsSystem/Stats/BP_Stat_Stamina.BP_Stat_Stamina_C")) (delegate `EndCondition`)))))

(event `/Game/Blueprints/MyGameSystem/Character/BPI_PlayerControllable.InputStartJumping`
  (bind _returnvalue (`|GenericCreateObject` "/Game/Blueprints/MyGameSystem/ConditionSystem/Conditions/BP_Condition_Standing.BP_Condition_Standing_C" (`self.GetConditionComponent`)))
  (`self.ChangeCondition` _returnvalue))

(event `EndCondition`
  (bind _returnvalue (`|GenericCreateObject` "/Game/Blueprints/MyGameSystem/ConditionSystem/Conditions/BP_Condition_Standing.BP_Condition_Standing_C" (`self.GetConditionComponent`)))
  (`self.ChangeCondition` _returnvalue))