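; Game mode for MyGameSystem that saves and loads the player character through a PartialSaveGame object in a single slot.
; SaveGame creates a save object, captures the character actor with its Save function and writes it to the slot.
; LoadGame unpossesses and destroys the current character, calls Load on the slot's save, then has the stored controller possess the character it finds afterwards.
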(event `SaveGame`
  (bind _returnvalue (`GameplayStatics.GetActorOfClass` "/Game/Blueprints/MyGameSystem/Character/BP_MyGameSystemCharacter.BP_MyGameSystemCharacter_C"))
  (bind _returnvalue_2 (`GameplayStatics.CreateSaveGameObject` "/Script/MySaveSystemPlugin.PartialSaveGame"))
  (`PartialSaveGame.Save` _returnvalue_2 (`|MakeArray` _returnvalue :!type "Object Object Reference"))
  (`GameplayStatics.SaveGameToSlot` _returnvalue_2 "1"))

(event `LoadGame`
  (bind _returnvalue (`GameplayStatics.GetActorOfClass` "/Game/Blueprints/MyGameSystem/Character/BP_MyGameSystemCharacter.BP_MyGameSystemCharacter_C"))
  (bind _output_get (set `self.ControllerToUpdate` (`Pawn.GetController` _returnvalue)))
  (`Controller.UnPossess` _output_get)
  (`self.K2_DestroyActor` _returnvalue)
  (bind _returnvalue_2 (`GameplayStatics.LoadGameFromSlot` "1"))
  (bind _aspartial_save_game (cast `PartialSaveGame` _returnvalue_2))
  (`PartialSaveGame.Load` _aspartial_save_game)
  (bind _returnvalue_3 (`GameplayStatics.GetActorOfClass` "/Game/Blueprints/MyGameSystem/Character/BP_MyGameSystemCharacter.BP_MyGameSystemCharacter_C"))
  (`Controller.Possess` (`self.ControllerToUpdate`) _returnvalue_3))

(fn `UserConstructionScript`)